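; Ambient bird character that idly hops around its spawn point and flies away when the player overlaps it.
; After a random start delay, a polling loop randomly turns it, steering back toward the start if it strays, then calls Move.
; Move sets flying movement mode and forwards to the bird Animation Blueprint's Move.
; The first player overlap stops the wandering and runs a timeline that interpolates it upward, then destroys it.
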(event EventActorBeginOverlap
  (params (OtherActor :type Actor%20Object%20Reference))
  (bind _returnvalue (Transformation|GetWorldLocation))
  (bind (_x _y _z) (Math|Vector|BreakVector _returnvalue))
  (if (Actor|ActorHasTag OtherActor "Player")
    (Utilities|FlowControl|DoOnce false
      (:Completed
        (Variables|Default|SetFlying true)
        (bind _speed (Timeline|Fly%20away PlayFromStart)
          (:Update
            (Transformation|SetActorLocation (Math|Interpolation|VInterpTo _returnvalue (Math|Vector|MakeVector _x _y (+ _z 5e+02)) 0.2 _speed) false))
          (:Finished
            (Actor|DestroyActor)))))))

(event EventBeginPlay
  (Utilities|FlowControl|Delay (Math|Random|RandomFloatinRange 0.0 2.0))
  (CallFunction|Move)
  (Utilities|FlowControl|Sequence
    (:then_0
      (Variables|Default|SetStartlocation (Transformation|GetWorldLocation)))
    (:then_1
      (if (and (== (Math|Random|RandomInteger 6) 5) (not (Variables|Default|GetFlying))) :!label _label
        (Utilities|FlowControl|Sequence
          (:then_0
            (Variables|Default|SetStraying (>= (Math|Vector|VectorLength (- (Variables|Default|GetStartlocation) (Transformation|GetWorldLocation))) 5e+01))
            (if (Variables|Default|GetStraying)
              (Transformation|SetActorRelativeRotation (Class|KismetMathLibrary|MakeRot 0.0 (.Yaw (Class|KismetMathLibrary|BreakRot (Math|Conversions|RotationFromXVector (- (Variables|Default|GetStartlocation) (Transformation|GetWorldLocation))))) 0.0))
              (else
                (Variables|Default|SetRandomTurn (Class|KismetMathLibrary|MakeRot 0.0 (.Yaw (Class|KismetMathLibrary|BreakRot (Math|Random|RandomRotator false))) 0.0))
                (Transformation|SetActorRelativeRotation (Variables|Default|GetRandomTurn)))))
          (:then_1
            (CallFunction|Move)
            (goto _label)))
        (else
          (Utilities|FlowControl|Delay 1.0)
          (goto _label))))))

(fn ConstructionScript)

(fn Move
  (Pawn|Components|CharacterMovement|SetMovementMode "MOVE_Flying" 0)
  (bind _asbp_bird_animbluprint (Utilities|Casting|CastToBp_Bird_animbluprint (Components|SkeletalMesh|GetAnimInstance (Variables|Character|GetMesh))))
  (Default|Move _asbp_bird_animbluprint))