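; Knife slit ("Fente") effect actor that animates left wool, right wool and bloody paper pieces, then destroys itself.
; BeginPlay runs three chained timelines: FenteLife, FenteDeath with its length set by FenteDeathLength, and Fentedestroy.
; FenteLife's end starts looping idle animations and FenteDeath together.
; Each FenteDeath update, rather than its finish, replays the vanish animations and triggers Fentedestroy, whose end destroys the actor.
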(event EventBeginPlay
  (Timeline|fenteLife Play
    (:Finished
      (Components|Animation|PlayAnimation (Variables|Default|GetLeftWool) "/Game/Animations/Asset_anim/A_leftwool_knife_Idle_fx.A_leftwool_knife_Idle_fx" true)
      (Components|Animation|PlayAnimation (Variables|Default|GetRightWool) "/Game/Animations/Asset_anim/A_rightwool_knife_Idle_fx.A_rightwool_knife_Idle_fx" true)
      (Components|Animation|PlayAnimation (Variables|Default|GetBloodyPaper) "/Game/Animations/Asset_anim/A_bloodypaper_knife_Idle_fx.A_bloodypaper_knife_Idle_fx" true)
      (Components|Timeline|SetTimelineLength (Variables|Default|GetfenteDeathLength))
      (Timeline|fenteDeath PlayFromStart
        (:Update
          (Components|Animation|PlayAnimation (Variables|Default|GetLeftWool) "/Game/Animations/Asset_anim/A_leftwool_knife_vanish_fx.A_leftwool_knife_vanish_fx" false)
          (Components|Animation|PlayAnimation (Variables|Default|GetRightWool) "/Game/Animations/Asset_anim/A_rightwool_knife_vanish_fx.A_rightwool_knife_vanish_fx" false)
          (Components|Animation|PlayAnimation (Variables|Default|GetBloodyPaper) "/Game/Animations/Asset_anim/A_bloodypaper_knife_vanish_fx.A_bloodypaper_knife_vanish_fx" false)
          (Timeline|fentedestroy Play
            (:Finished
              (Actor|DestroyActor))))))))

(fn ConstructionScript)