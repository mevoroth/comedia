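; BP_DialogSubs shows timed dialog subtitles by writing lines to the SubString variable of BP_HUD.
; StartDialogSubs sets a flag that lets Tick accumulate elapsed time and step an index through the Timestamps array.
; Timestamps alternate on and off: an even index that has been reached shows DialogLines at half that index, otherwise the subtitle is cleared.
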(event EventTick
  (params (DeltaSeconds :type Float%20%28single-precision%29))
  (bind _returnvalue (Game|GetPlayerController 0))
  (bind _timestamps (Variables|[Comedia]DialogSubs|GetTimestamps))
  (bind _returnvalue_2 (HUD|GetHUD _returnvalue))
  (if (Variables|Default|GetDialogStarted)
    (Variables|Default|SetElapsedTime (+ (Variables|Default|GetElapsedTime) DeltaSeconds))
    (Utilities|FlowControl|Sequence
      (:then_0
        ;[1 1 1] Increment timestamp index
        (if (and (< (Variables|Default|GetIndexTimestamp) (- (Utilities|Array|Length _timestamps) 1)) (> (Variables|Default|GetElapsedTime) (Utilities|Array|Get(acopy) _timestamps (+ (Variables|Default|GetIndexTimestamp) 1))))
          (Variables|Default|SetIndexTimestamp (+ (Variables|Default|GetIndexTimestamp) 1))))
      (:then_1
        (if (and (== (Math|Integer|%(Integer) (Variables|Default|GetIndexTimestamp) 2) 0) (> (Variables|Default|GetElapsedTime) (Utilities|Array|Get(acopy) (Variables|[Comedia]DialogSubs|GetTimestamps) (Variables|Default|GetIndexTimestamp))))
          (bind _asbp_hud (Utilities|Casting|CastToBP_HUD _returnvalue_2))
          (Variables|/Game/Blueprints/BP_HUD.BP_HUD_C|SetSubString _asbp_hud (Utilities|Array|Get(acopy) (Variables|[Comedia]DialogSubs|GetDialogLines) (/ (Variables|Default|GetIndexTimestamp) 2)))
          (else
            (bind _asbp_hud_2 (Utilities|Casting|CastToBP_HUD _returnvalue_2))
            ;[1 1 1] Set empty string
            (if (!= (Utilities|String|Len (Variables|/Game/Blueprints/BP_HUD.BP_HUD_C|GetSubString _asbp_hud_2)) 0)
              (Variables|/Game/Blueprints/BP_HUD.BP_HUD_C|SetSubString _asbp_hud_2 ""))))))))

(fn ConstructionScript)

(fn StartDialogSubs
  (Variables|Default|SetDialogStarted true))