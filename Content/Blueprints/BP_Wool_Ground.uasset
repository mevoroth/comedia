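; Wool ground actor that feeds the player character's foot position to its wool material for footstep effects.
; Each Tick creates a new dynamic instance of M_Wool_Inst and sets X, Y and depth parameters for left and right feet.
; Socket position relative to the actor maps to inverted coordinates over a 20000-unit square, with depth fading by height against ThresholdFootStep.
; Both left and right parameters read LFootSocket, so they receive identical values.
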(event EventTick
  (params (DeltaSeconds :type Float%20%28single-precision%29))
  (bind _returnvalue (Game|GetPlayerCharacter 0))
  (bind _returnvalue_2 (Transformation|GetActorLocation))
  (bind _thresholdfootstep (Variables|Default|GetThresholdFootStep))
  (bind _returnvalue_3 (Transformation|GetSocketLocation _returnvalue "LFootSocket"))
  (bind _returnvalue_4 (Transformation|GetSocketLocation _returnvalue "LFootSocket"))
  (bind _returnvalue_5 (- _returnvalue_3 _returnvalue_2))
  (bind _returnvalue_6 (- _returnvalue_4 _returnvalue_2))
  (bind _returnvalue_7 (+ _returnvalue_5 "10000.000000,10000.000000, 0"))
  (bind _returnvalue_8 (+ _returnvalue_6 "10000.000000,10000.000000, 0"))
  (bind (_x _y _z) (Math|Vector|BreakVector _returnvalue_7))
  (bind (_x_2 _y_2 _z_2) (Math|Vector|BreakVector _returnvalue_8))
  (bind _returnvalue_9 (Rendering|Material|CreateDynamicMaterialInstance 0 "/Game/Materials/M_Wool_Inst.M_Wool_Inst" :!class /Script/Engine.PrimitiveComponent))
  (Rendering|Material|SetScalarParameterValue _returnvalue_9 "LeftX" (- 1.0 (/ _x_2 2e+04)) :!class /Script/Engine.MaterialInstanceDynamic)
  (Rendering|Material|SetScalarParameterValue _returnvalue_9 "LeftY" (- 1.0 (/ _y_2 2e+04)) :!class /Script/Engine.MaterialInstanceDynamic)
  (Rendering|Material|SetScalarParameterValue _returnvalue_9 "LeftDepthFootStep" (- 1.0 (Math|Float|Clamp(Float) (/ _z_2 _thresholdfootstep))) :!class /Script/Engine.MaterialInstanceDynamic)
  (Rendering|Material|SetScalarParameterValue _returnvalue_9 "RightX" (- 1.0 (/ _x 2e+04)) :!class /Script/Engine.MaterialInstanceDynamic)
  (Rendering|Material|SetScalarParameterValue _returnvalue_9 "RightY" (- 1.0 (/ _y 2e+04)) :!class /Script/Engine.MaterialInstanceDynamic)
  (Rendering|Material|SetScalarParameterValue _returnvalue_9 "RightDepthFootStep" (- 1.0 (Math|Float|Clamp(Float) (/ _z _thresholdfootstep))) :!class /Script/Engine.MaterialInstanceDynamic))

(fn ConstructionScript)