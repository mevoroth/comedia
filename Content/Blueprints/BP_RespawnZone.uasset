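; BP_RespawnZone is a checkpoint trigger that registers itself as the player's current respawn zone.
; On actor overlap, it checks that the other actor is player character 0, then casts it to LiyaCharacter and sets CurrentRespawnZone to itself.
; A Triggered flag makes this one-shot, so re-entering an earlier zone does not make it current again.
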(event EventActorBeginOverlap
  (params (OtherActor :type Actor%20Object%20Reference))
  ;[1 1 1] Set current respawn zone when triggered
  (if (and (== (Game|GetPlayerCharacter 0) OtherActor) (not (Variables|Default|GetbTriggered)))
    (Variables|Default|SetbTriggered true)
    (bind _asliya_character (Utilities|Casting|CastToLiyaCharacter (Game|GetPlayerCharacter 0)))
    (Variables|/Script/Comedia.LiyaCharacter|SetCurrentRespawnZone _asliya_character self)))

(fn ConstructionScript)