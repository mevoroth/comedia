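; BP_TriggerSwitchcalls is a trigger actor that changes the Wwise "Liyacalls" audio switch group on the player character.
; When the player begins overlapping it, it sets the group to the state named by its Switch variable.
; When the player stops overlapping, it sets the group to the state named by SwitchBack.
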(event EventActorBeginOverlap
  (params (OtherActor :type Actor%20Object%20Reference))
  (bind _returnvalue (Game|GetPlayerCharacter 0))
  (if (== OtherActor _returnvalue)
    (Class|AkGameplayStatics|SetSwitch "Liyacalls" (Utilities|String|StringToName (Variables|[Comedia]Switchcall|GetSwitch)) _returnvalue)))

(event EventActorEndOverlap
  (params (OtherActor :type Actor%20Object%20Reference))
  (bind _returnvalue (Game|GetPlayerCharacter 0))
  (if (== OtherActor _returnvalue)
    (Class|AkGameplayStatics|SetSwitch "Liyacalls" (Utilities|String|StringToName (Variables|[Comedia]Switchcall|GetSwitch_back)) _returnvalue)))

(fn ConstructionScript)