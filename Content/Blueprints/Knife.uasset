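; Knife actor with animation, audio and camera feedback around the player, building on a parent class's Tick.
; It plays a spawn animation on construction, then starts a looping Wwise sound and, after a short delay, a looping animation.
; Tick triggers a one-time flyby whoosh and repeated camera shakes within distance thresholds, with shake scale increasing with distance.
; OnKnifeDestroy disables collision, plays a vanish animation and destroys the actor when the Vanish timeline finishes.
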(event EventOnKnifeDestroy
  (Utilities|FlowControl|DoOnce false
    (:Completed
      (Collision|SetActorEnableCollision false)
      (Components|Animation|PlayAnimation (Variables|Character|GetMesh) "/Game/Animations/Asset_anim/A_knife_Vanish.A_knife_Vanish" false)
      (Timeline|Vanish PlayFromStart
        (:Finished
          (Actor|DestroyActor))))))

(event EventTick
  (params (DeltaSeconds :type Float%20%28single-precision%29))
  (bind _returnvalue (Game|GetPlayerCharacter 0))
  (bind _distancecamerashake (Variables|Default|GetDistanceCameraShake))
  ;[1 1 1] Knife woosh if d < 250
  (|CallParentFunction 0.0)
  (Utilities|FlowControl|Sequence
    (:then_0
      (if (not (Variables|Default|GetHasWooshed))
        (bind _returnvalue_2 (Transformation|GetDistanceTo _returnvalue))
        (Math|Float|CompareFloat _returnvalue_2 (Variables|Default|GetDistanceWoosh)
          (:<
            (Class|AkGameplayStatics|PostEvent "/Game/Audio/SFX/Knife_Flyby.Knife_Flyby" self true)
            (Variables|Default|SetHasWooshed true)))))
    (:then_1
      ;[1 1 1] Camera shake knife next to character
      (bind _returnvalue_3 (Transformation|GetDistanceTo _returnvalue))
      (Math|Float|CompareFloat _returnvalue_3 _distancecamerashake
        (:<
          (Class|PlayerController|ClientPlayCameraShake (Game|GetPlayerController 0) "/Game/Blueprints/BP_CameraShake.BP_CameraShake_C" (* (/ _returnvalue_3 _distancecamerashake) 0.25) "CameraLocal" "0, 0, 0"))))))

(event EventBeginPlay
  ;[1 1 1] Knife continuous sound ( distance variable)
  (Class|AkGameplayStatics|PostEvent "/Game/Audio/SFX/Knife_Loop_Start.Knife_Loop_Start" self true)
  (Utilities|FlowControl|Delay 0.4)
  (Components|Animation|PlayAnimation (Variables|Character|GetMesh) "/Game/Animations/Asset_anim/Sk_knife_Anim.Sk_knife_Anim" true))

(fn ConstructionScript
  (Components|Animation|PlayAnimation (Variables|Character|GetMesh) "/Game/Animations/Asset_anim/A_knife_spawn.A_knife_spawn" false))