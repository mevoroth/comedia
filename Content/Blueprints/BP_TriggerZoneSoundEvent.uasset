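; One-shot trigger zone that plays Wwise sound events and dialog subtitles when the player character first overlaps it.
; It posts the main event on the player and, if set, a second event on a chosen actor, then starts the subtitles if a subs object is assigned.
; For a non-zero duration, it holds DialogRunning on LiyaCharacter so the Prince does not call during dialog.
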(event EventActorBeginOverlap
  (params (OtherActor :type Actor%20Object%20Reference))
  (bind _returnvalue (Game|GetPlayerCharacter 0))
  (bind _subsdialogs (Variables|[Comedia]TriggerZoneSoundEvent|GetSubsDialogs))
  (bind _eventduration (Variables|[Comedia]TriggerZoneSoundEvent|GetEventDuration))
  (bind _secondsoundeventtolaunch (Variables|[Comedia]TriggerZoneSoundEvent|GetSecondSoundEventToLaunch))
  (bind _secondsoundeventactor (Variables|[Comedia]TriggerZoneSoundEvent|GetSecondSoundEventActor))
  ;[1 1 1] Trigger and check for first launch
  (if (and (== OtherActor _returnvalue) (not (Variables|Default|GetSoundEventLaunched)))
    (Variables|Default|SetSoundEventLaunched true)
    (Utilities|FlowControl|Sequence
      (:then_0
        ;[1 1 1] Post first event on player character
        (Class|AkGameplayStatics|PostEvent (Variables|[Comedia]TriggerZoneSoundEvent|GetEventToLaunch) _returnvalue false)
        ;[1 1 1] Set bDialogRunning on player character to avoid Prince calling during dialog
        (if (!= _eventduration 0.0)
          (bind _asliya_character (Utilities|Casting|CastToLiyaCharacter (Game|GetPlayerCharacter 0)))
          (Variables|/Script/Comedia.LiyaCharacter|SetbDialogRunning _asliya_character true)
          (Utilities|FlowControl|Delay _eventduration)
          (Variables|/Script/Comedia.LiyaCharacter|SetbDialogRunning _asliya_character false)))
      (:then_1
        ;[1 1 1] Post second sound event on selected actor
        (if (and (Utilities|IsValid _secondsoundeventtolaunch) (Utilities|IsValid _secondsoundeventactor))
          (Class|AkGameplayStatics|PostEvent _secondsoundeventtolaunch _secondsoundeventactor false)))
      (:then_2
        ;[1 1 1] Start subs
        (Utilities|IsValid _subsdialogs
          (:Is%20Valid
            (Default|StartDialogSubs _subsdialogs)))))))

(fn ConstructionScript)