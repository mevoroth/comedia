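; Grabbable poster actor with two grip points that can act as a timed fire hazard, shown by a decal.
; Head and tail overlaps and the Use input feed range and grab functions, while Tick updates grip locations.
; With both timers non-zero, the decal blinks; while visible, a player in fire range triggers a death Matinee, then respawns after a delay.
; A dynamic material instance receives the poster's forward vector at BeginPlay.
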(event OnComponentEndOverlap(GripHead)
  (params (OtherActor :type Actor%20Object%20Reference) (OtherComp :type Primitive%20Component%20Object%20Reference) (OtherBodyIndex :type Integer))
  (Class|PosterActor|OutRange))

(event OnComponentEndOverlap(GripTail)
  (params (OtherActor :type Actor%20Object%20Reference) (OtherComp :type Primitive%20Component%20Object%20Reference) (OtherBodyIndex :type Integer))
  (Class|PosterActor|OutRange))

(event OnComponentBeginOverlap(GripHead)
  (params (OtherActor :type Actor%20Object%20Reference) (OtherComp :type Primitive%20Component%20Object%20Reference) (OtherBodyIndex :type Integer) (bFromSweep :type Boolean) (SweepResult :type Hit%20Result%20Structure%20%28by%20ref%29))
  (Class|PosterActor|InRange true))

(event OnComponentBeginOverlap(GripTail)
  (params (OtherActor :type Actor%20Object%20Reference) (OtherComp :type Primitive%20Component%20Object%20Reference) (OtherBodyIndex :type Integer) (bFromSweep :type Boolean) (SweepResult :type Hit%20Result%20Structure%20%28by%20ref%29))
  (Class|PosterActor|InRange false))

(event EventTick
  (params (DeltaSeconds :type Float%20%28single-precision%29))
  (bind _decal (Variables|Default|GetDecal))
  (CallFunction|UpdateGripsLocation)
  (if (and (!= (Variables|[Comedia]Poster|GetTimeOff) 0.0) (!= (Variables|[Comedia]Poster|GetTimeOn) 0.0))
    (Utilities|FlowControl|Sequence
      (:then_0
        ;[1 1 1] Detect  player killed
        (if (Variables|[Comedia]Poster|GetIsOff)
          (if (Class|PosterActor|IsinFireRange (Transformation|GetActorLocation (Game|GetPlayerCharacter 0)))
            (if (not (Variables|[Comedia]Poster|GetPlayerKilled))
              (Variables|[Comedia]Poster|SetPlayerKilled true)
              (Audio|Components|Audio|Play (Variables|[Comedia]Poster|GetMatineePlayerKilled))
              (Utilities|FlowControl|Delay 1.2)
              (Transformation|SetActorLocation (Game|GetPlayerCharacter 0) (Transformation|GetActorLocation (Variables|[Comedia]Poster|GetRespawnPoint)) false))
            (else
              (Variables|[Comedia]Poster|SetPlayerKilled false)))))
      (:then_1
        ;[1 1 1] Decale state switching
        (Variables|[Comedia]Poster|SetElapsedTime (- (Variables|[Comedia]Poster|GetElapsedTime) DeltaSeconds))
        (Math|Float|CompareFloat (Variables|[Comedia]Poster|GetElapsedTime) 0.0
          (:==
            _)
          (:<
            _))
        (Variables|[Comedia]Poster|SetIsOff (not (Variables|[Comedia]Poster|GetIsOff)))
        (if (Variables|[Comedia]Poster|GetIsOff)
          (Variables|[Comedia]Poster|SetElapsedTime (Variables|[Comedia]Poster|GetTimeOn))
          (else
            (Variables|[Comedia]Poster|SetElapsedTime (Variables|[Comedia]Poster|GetTimeOff)))))
      (:then_2
        ;[1 1 1] Toggle decal visibility
        (if (or (and (Variables|[Comedia]Poster|GetIsOff) (not (Rendering|IsVisible (Variables|Default|GetDecal)))) (and (not (Variables|[Comedia]Poster|GetIsOff)) (Rendering|IsVisible (Variables|Default|GetDecal))))
          (Rendering|ToggleVisibility (Variables|Default|GetDecal) false))))
    (elif (Rendering|IsVisible _decal)
      (Rendering|ToggleVisibility _decal true))))

(event EventBeginPlay
  (|CallParentFunction)
  ;[1 1 1] Enable Input
  (Input|EnableInput (Game|GetPlayerController 0))
  (bind _returnvalue (Rendering|Material|CreateDynamicMaterialInstance 0 0 :!class /Script/Engine.PrimitiveComponent))
  (Rendering|Material|SetVectorParameterValue _returnvalue "PosterForward" (Math|Conversions|ToLinearColor(Vector) (Class|PosterActor|GetPosterForward)) :!class /Script/Engine.MaterialInstanceDynamic))

(event Input|ActionEvents|InputActionUse
  (:Pressed
    (Class|PosterActor|Grabbing true))
  (:Released
    (Class|PosterActor|Grabbing false)))

(fn ConstructionScript)

(fn GetGripTail
  (return (Transformation|GetWorldLocation (Variables|Default|GetGripTail))))

(fn GetGripHead
  (return (Transformation|GetWorldLocation (Variables|Default|GetGripHead))))

(fn UpdateGripsLocation
  (Transformation|SetWorldLocation (Variables|Default|GetGripHead) (Class|PosterActor|GetGripHeadUpdated) false)
  (Transformation|SetWorldLocation (Variables|Default|GetGripTail) (Class|PosterActor|GetGripTailUpdated) false))