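; BP_Tempest_FX is a tempest effect Blueprint that animates eight Tempest components through continuous layered rotation.
; Each Tick adds a local spin to itself, then smaller offsets to two component groups in opposite directions about the same axis.
; A third group receives zero added rotation.
; Steps are fixed per frame without delta-time scaling, so spin speed follows frame rate.
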(event EventTick
  (params (DeltaSeconds :type Float%20%28single-precision%29))
  (Transformation|AddLocalRotation "0,1.000000, 0" false)
  (Transformation|AddLocalRotation (Variables|Default|Gettempest1) "0,0.500000, 0" false)
  (Transformation|AddLocalRotation (Variables|Default|Gettempest6) "0,0.000000, 0" false)
  (Transformation|AddLocalRotation (Variables|Default|Gettempest8) "0,-0.200000, 0" false))

(fn ConstructionScript)